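; Gameplay game mode Blueprint that bootstraps a roguelite run when play begins.
; On BeginPlay it has the Roguelite subsystem load and register its actions.
; If no run is active, it starts a new run and acquires one stack of each action in its default action list.
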(event `self.ReceiveBeginPlay`
  (`parent.ReceiveBeginPlay`)
  (`RogueliteSubsystem.LoadAndRegisterActions` (subsystem `RogueliteSubsystem`) "RogueliteActionData")
  (if (not (`RogueliteSubsystem.IsRunActive` (subsystem `RogueliteSubsystem`)))
    (`RogueliteBlueprintLibrary.StartRun`)
    (for _array_element (`self.DefaultActions`)
      (`RogueliteBlueprintLibrary.AcquireAction` _array_element))))

(fn `UserConstructionScript`)