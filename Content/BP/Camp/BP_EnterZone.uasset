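; Camp trigger zone that sends the player into L_Gameplay, provided a primary weapon is equipped.
; When a PRPlayerCharacter overlaps the Box, it queries that character's equipment manager for the primary weapon slot.
; With a weapon, the camera fades out and the level opens after a short delay.
; Without one, it pushes a W_Modal with a Korean message saying a weapon must be equipped.
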(event `self.Box.OnComponentBeginOverlap`
  (params (OverlappedComponent :type "PrimitiveComponent Object Reference") (OtherActor :type "Actor Object Reference") (OtherComp :type "PrimitiveComponent Object Reference") (OtherBodyIndex :type Integer) (bFromSweep :type Boolean) (SweepResult :type "HitResult Structure (by ref)"))
  (bind _asprplayer_character (cast `PRPlayerCharacter` OtherActor))
  (bind _returnvalue (`PREquipmentBlueprintLibrary.GetEquipmentManager` _asprplayer_character))
  (`/Engine/EditorBlueprintResources/StandardMacros.IsValid` _returnvalue
    (:`Is Valid`
      (if (`PREquipmentManagerComponent.HasEquipment` _returnvalue (struct :`TagName` "Equipment.Slot.Weapon.Primary"))
        (`PlayerCameraManager.StartCameraFade` :`self` (`GameplayStatics.GetPlayerCameraManager` 0) :`FromAlpha` 0.0 :`ToAlpha` 1.0 :`Duration` 0.3 :`bHoldWhenFinished` true)
        (`KismetSystemLibrary.Delay` 1.0)
        (`GameplayStatics.OpenLevelBySoftObjectPtr` "/Game/Maps/L_Gameplay.L_Gameplay")
        (else
          (bind _returnvalue_2 (`PRUIBlueprintLibrary.PushUI` (`GameplayStatics.GetPlayerController` 0) "/Game/UI/Modal/W_Modal.W_Modal_C"))
          (`/Engine/EditorBlueprintResources/StandardMacros.IsValid` _returnvalue_2
            (:`Is Valid`
              (`/Game/UI/Modal/W_Modal.SetText` _returnvalue_2 "무기를 장착해야 합니다!"))))))))

(fn `UserConstructionScript`)