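; BP_AttackTraceTestActor is a test actor that periodically fires a BP_PlasmaWave along its forward vector.
; A looping timer started on BeginPlay spawns the wave at the actor's transform.
; It then initializes the wave with a dodgeable damage GameplayEffect spec, built from the player character's own Ability System Component with SetByCaller damage.
; A debug-drawn capsule trace that notifies combat-interface hits remains in the graph but never runs.
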(event `CustomEvent`
  (bind _returnvalue (`GameplayStatics.GetPlayerCharacter` 0))
  (bind _returnvalue_2 (`AbilitySystemBlueprintLibrary.GetAbilitySystemComponent` _returnvalue))
  (bind _returnvalue_3 (`|SpawnActorFromClass` "/Game/BP/Ability/Leviathan/BP_PlasmaWave.BP_PlasmaWave_C" (`self.GetTransform`) "Undefined" "MultiplyWithRoot" null null))
  (`/Engine/EditorBlueprintResources/StandardMacros.IsValid` _returnvalue
    (:`Is Valid`
      (`/Engine/EditorBlueprintResources/StandardMacros.IsValid` _returnvalue_2
        (:`Is Valid`
          (bind _returnvalue_4 (`AbilitySystemBlueprintLibrary.AssignTagSetByCallerMagnitude` (`AbilitySystemComponent.MakeOutgoingSpec` _returnvalue_2 "/Game/BP/Ability/Common/GE_Damage_Dodgeable.GE_Damage_Dodgeable_C" 0.0 (`AbilitySystemComponent.MakeEffectContext` _returnvalue_2)) (struct :`TagName` "SetByCaller.Combat.Damage") 10.0))
          (`PRPlasmaWave.InitWave` _returnvalue_3 (`self.GetActorForwardVector`) _returnvalue_4))))))

(event `self.ReceiveBeginPlay`
  (`KismetSystemLibrary.K2_SetTimerDelegate` (delegate `CustomEvent`) 2.0 true))

(fn `UserConstructionScript`)