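; Boss death gameplay ability that finalizes a boss's death and records the kill.
; On OnDeathFinished, it pauses the avatar's mesh animations, disables character movement and stops the StateTree logic on its PRAIController.
; It then calls FinishDie and increments the Event.Kill.Boss count on the gameplay game state.
; ActivateAbility and OnEndAbility are empty here, so this graph handles only the post-death step.
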(event `self.K2_OnDeathFinished`
  (bind _charactermovement (`Character.CharacterMovement` (`self.Character`)))
  (`|ExecutionSequence`
    (:`then_0`
      (bind _ascharacter (cast `Character` (`self.GetAvatarActorFromActorInfo`)))
      (set `self.Character` _ascharacter)
      (set `SkeletalMeshComponent.bPauseAnims` true (`Character.Mesh` _ascharacter))
      (`|ExecutionSequence`
        (:`then_0`
          (`/Engine/EditorBlueprintResources/StandardMacros.IsValid` _charactermovement
            (:`Is Valid`
              (`CharacterMovementComponent.SetMovementMode` _charactermovement "MOVE_None" 0))))
        (:`then_1`
          (bind _aspraicontroller (cast `PRAIController` (`AIBlueprintHelperLibrary.GetAIController` (`self.Character`))))
          (bind _statetreecomponent (`PRAIController.StateTreeComponent` _aspraicontroller))
          (if (`BrainComponent.IsRunning` _statetreecomponent)
            (`BrainComponent.StopLogic` _statetreecomponent "")))
        (:`then_2`
          (`self.FinishDie`))
        (:`then_3`
          (bind _asprgameplay_game_state (cast `PRGameplayGameState` (`GameplayStatics.GetGameState`)))
          (`PRGameplayGameState.AddEventCount` _asprgameplay_game_state (`BlueprintGameplayTagLibrary.MakeLiteralGameplayTag` (struct :`TagName` "Event.Kill.Boss")) 1))))))