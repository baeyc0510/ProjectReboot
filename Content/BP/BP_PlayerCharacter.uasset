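; BP_PlayerCharacter is the player character Blueprint, with a test hook that opens a roguelite equipment choice panel on the E key.
; Pressing E creates W_ActionDecisionPanel, switches to UI-only input with the mouse cursor shown, and passes the character and BP_PreviewCharacter class as preview source.
; A roguelite query for three Equipment-tagged entries then fills the panel's decision list.
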(event `self.ReceiveBeginPlay`
  (`parent.ReceiveBeginPlay`))

(event `Key|E`
  (params (Key :type "Key Structure"))
  (bind _returnvalue (`GameplayStatics.GetPlayerController` 0))
  (:`Pressed`
    (bind _returnvalue_2 (`|CreateWidget` "/Game/BP/UI/W_ActionDecisionPanel.W_ActionDecisionPanel_C"))
    (bind _output_get (set `self.TestDecisionPanel` _returnvalue_2))
    (`UserWidget.AddToViewport` _output_get 0)
    (`WidgetBlueprintLibrary.SetInputMode_UIOnlyEx` _returnvalue null)
    (set `PlayerController.bShowMouseCursor` true _returnvalue)
    (`PRActionDecisionPanel.SetSourceActor` (`self.TestDecisionPanel`) self "/Game/BP/BP_PreviewCharacter.BP_PreviewCharacter_C")
    (bind _returnvalue_3 (`RogueliteBlueprintLibrary.ExecuteQuery` (make `RogueliteQuery` (struct :`GameplayTags` (struct :`(TagName` "Equipment"))) 3)))
    (`PRActionDecisionPanel.SetDecisionList` (`self.TestDecisionPanel`) _returnvalue_3)))

(fn `UserConstructionScript`)