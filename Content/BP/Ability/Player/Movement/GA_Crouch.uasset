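; GA_Crouch is a player movement Gameplay Ability that acts as a crouch toggle.
; On activation it applies the CrouchGE gameplay effect to the owner and stores the handle.
; A WaitInputPress task ends the ability on the next input press.
; On end it removes the effect through the stored handle and ends the input task if still valid.
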(event `self.K2_ActivateAbility`
  (bind _returnvalue (`self.K2_ApplyGameplayEffectSpecToOwner` (`self.MakeOutgoingGameplayEffectSpec` (`self.CrouchGE`))))
  (set `self.ActiveCrouchEffectHandle` _returnvalue)
  (bind _asynctaskproxy (`AbilityTask_WaitInputPress.WaitInputPress` false)
    (:`then`
      (set `self.InputTask` _asynctaskproxy))
    (:`OnPress`
      (`self.K2_EndAbility`))))

(event `self.K2_OnEndAbility`
  (params (bWasCancelled :type Boolean))
  (`self.BP_RemoveGameplayEffectFromOwnerWithHandle` (`self.ActiveCrouchEffectHandle`))
  (bind _inputtask (`self.InputTask`)
    (:`then`
      (`GameplayTask.EndTask` _inputtask))
    (:`else`)))