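; BP_TestModularEquipment is a test actor that assembles a modular equipment item in its construction script.
; Each construction run uninitializes any existing EquipmentInstance, then constructs a new one and initializes it on the root component with PrimaryActionData.
; It then attaches every entry in PartActionDataList as a part.
; The event graph holds only disabled placeholder events, so there is no gameplay logic.
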(fn `UserConstructionScript`
  (`|ExecutionSequence`
    (:`then_0`
      (bind _equipmentinstance (`self.EquipmentInstance`)
        (:`then`
          (`EquipmentInstance.Uninitialize` _equipmentinstance))
        (:`else`)))
    (:`then_1`
      (bind _returnvalue (`|GenericCreateObject` "/Script/ProjectReboot.EquipmentInstance"))
      (bind _output_get (set `self.EquipmentInstance` _returnvalue))
      (`/Engine/EditorBlueprintResources/StandardMacros.IsValid` _output_get
        (:`Is Valid`
          (`EquipmentInstance.Initialize` (`self.EquipmentInstance`) (`self.DefaultSceneRoot`) (`self.PrimaryActionData`))
          (for _array_element (`self.PartActionDataList`)
            (`EquipmentInstance.AttachPart` (`self.EquipmentInstance`) _array_element)))))))