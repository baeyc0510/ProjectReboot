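; Enemy death gameplay ability that handles kill feedback, loot and cleanup.
; Activation runs the parent logic, then shows a kill hit marker through the first player's crosshair view model.
; When death finishes, it freezes animation, movement and the AI StateTree, calls FinishDie and adds a dissolve cue.
; It also rolls a roguelite field drop, increments the run's kill count and destroys the avatar after a short delay.
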(event `self.K2_OnDeathFinished`
  (bind _returnvalue (`self.GetAvatarActorFromActorInfo`))
  (bind _charactermovement (`Character.CharacterMovement` (`self.Character`)))
  (`|ExecutionSequence`
    (:`then_0`
      (bind _ascharacter (cast `Character` (`self.GetAvatarActorFromActorInfo`)))
      (set `self.Character` _ascharacter)
      (set `SkeletalMeshComponent.bPauseAnims` true (`Character.Mesh` _ascharacter))
      (`|ExecutionSequence`
        (:`then_0`
          (`/Engine/EditorBlueprintResources/StandardMacros.IsValid` _charactermovement
            (:`Is Valid`
              (`CharacterMovementComponent.SetMovementMode` _charactermovement "MOVE_None" 0))))
        (:`then_1`
          (bind _aspraicontroller (cast `PRAIController` (`AIBlueprintHelperLibrary.GetAIController` (`self.Character`))))
          (bind _statetreecomponent (`PRAIController.StateTreeComponent` _aspraicontroller))
          (if (`BrainComponent.IsRunning` _statetreecomponent)
            (`BrainComponent.StopLogic` _statetreecomponent "")))
        (:`then_2`
          (`self.FinishDie`)
          (`self.K2_AddGameplayCue` (struct :`TagName` "GameplayCue.Character.Dissolve"))
          (`PRBlueprintFunctionLibrary.TrySpawnFieldDrop` (`Actor.K2_GetActorLocation` (`self.GetAvatarActorFromActorInfo`)) (make `RogueliteQuery` (struct :`GameplayTags` (struct :`(TagName` "FieldDrop") :`(TagName` "EnemyDrop")))) "/Game/BP/Stage/FieldDrops/BP_FieldDrop.BP_FieldDrop_C" 0.1))
        (:`then_3`
          (`KismetSystemLibrary.Delay` 3.0)
          (`/Engine/EditorBlueprintResources/StandardMacros.IsValid` _returnvalue
            (:`Is Valid`
              (`Actor.K2_DestroyActor` _returnvalue))))
        (:`then_4`
          (`RogueliteBlueprintLibrary.AddRogueliteStateValue` (struct :`TagName` "Event.Kill") 1.0))))))

(event `self.K2_ActivateAbility`
  (`parent.K2_ActivateAbility`)
  (bind _returnvalue (`PRUIBlueprintLibrary.GetOrCreateGlobalViewModel` (`GameplayStatics.GetPlayerController` 0) "/Script/ProjectReboot.PRCrosshairViewModel"))
  (`PRCrosshairViewModel.ShowHitMarker` _returnvalue "Kill"))