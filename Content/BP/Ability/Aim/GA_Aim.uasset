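; GA_Aim is a Gameplay Ability that toggles aiming down sights (ADS) by holding a gameplay effect on its owner.
; Activation applies the ADS effect, stores its handle and starts a WaitInputPress task, so the next input press ends the ability.
; On end, it removes the effect by that handle and ends the input task if still valid.
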(event `self.K2_ActivateAbility`
  (bind _returnvalue (`self.K2_ApplyGameplayEffectSpecToOwner` (`self.MakeOutgoingGameplayEffectSpec` (`self.ADSEffectClass`))))
  (set `self.ADSEffectHandle` _returnvalue)
  (bind _asynctaskproxy (`AbilityTask_WaitInputPress.WaitInputPress` false)
    (:`then`
      (set `self.WaitInputTask` _asynctaskproxy))
    (:`OnPress`
      (`self.K2_EndAbility`))))

(event `self.K2_OnEndAbility`
  (params (bWasCancelled :type Boolean))
  (`self.BP_RemoveGameplayEffectFromOwnerWithHandle` (`self.ADSEffectHandle`))
  (bind _waitinputtask (`self.WaitInputTask`)
    (:`then`
      (`GameplayTask.EndTask` _waitinputtask))
    (:`else`)))