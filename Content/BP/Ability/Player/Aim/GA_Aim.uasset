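; Gameplay ability that toggles aim-down-sights for the player.
; Activation applies the ADS gameplay effect to the owner and waits for another input press to end the ability.
; Ending removes the effect by its stored handle and stops the input task.
; Zoom in and out sounds play only when the equipment manager reports a primary weapon in its slot.
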(event `self.K2_ActivateAbility`
  (bind _returnvalue (`self.K2_ApplyGameplayEffectSpecToOwner` (`self.MakeOutgoingGameplayEffectSpec` (`self.ADSEffectClass`))))
  (set `self.ADSEffectHandle` _returnvalue)
  (`|ExecutionSequence`
    (:`then_0`
      (if (`self.HasWeapon`)
        (`GameplayStatics.PlaySound2D` "/Game/Audio/MetaSounds/sfx_ZoomIn_nl_meta_Preset.sfx_ZoomIn_nl_meta_Preset" 1.0 1.0 0.0 null null)))
    (:`then_1`
      (bind _asynctaskproxy (`AbilityTask_WaitInputPress.WaitInputPress` false)
        (:`then`
          (set `self.WaitInputTask` _asynctaskproxy))
        (:`OnPress`
          (`self.K2_EndAbility`))))))

(event `self.K2_OnEndAbility`
  (params (bWasCancelled :type Boolean))
  (`self.BP_RemoveGameplayEffectFromOwnerWithHandle` (`self.ADSEffectHandle`))
  (bind _waitinputtask (`self.WaitInputTask`)
    (:`then`
      (`GameplayTask.EndTask` _waitinputtask)
      (if (`self.HasWeapon`)
        (`GameplayStatics.PlaySound2D` "/Game/Audio/MetaSounds/sfx_ZoomOut_nl_meta_Preset.sfx_ZoomOut_nl_meta_Preset" 1.0 1.0 0.0 null null)))
    (:`else`)))

(fn `HasWeapon`
  (returns (ReturnValue :type Boolean))
  (bind _returnvalue (`PREquipmentBlueprintLibrary.GetEquipmentManager` (`self.GetAvatarActorFromActorInfo`)))
  (`/Engine/EditorBlueprintResources/StandardMacros.IsValid` _returnvalue
    (:`Is Valid`
      (return (`PREquipmentManagerComponent.HasEquipment` _returnvalue (struct :`TagName` "Equipment.Slot.Weapon.Primary"))))
    (:`Is Not Valid`
      (return false))))